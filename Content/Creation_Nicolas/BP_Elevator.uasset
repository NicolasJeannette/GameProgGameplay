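; BP_Elevator is an elevator actor that moves up or down one floor at a time.
; GoUp and GoDown pass a vertical direction to MoveToDirection and increment or decrement the CurrentEtage floor counter.
; MoveToDirection instantly offsets the actor's location by a fixed vertical step, with no sweep, interpolation or floor-limit check.
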(fn `GoDown`
  (`self.MoveToDirection` (* (`KismetMathLibrary.Vector_Up`) -1.0))
  (`/Engine/EditorBlueprintResources/StandardMacros.DecrementInt` (`self.CurrentEtage`)))

(fn `GoUp`
  (`self.MoveToDirection` (* (`KismetMathLibrary.Vector_Up`) 1.0))
  (`/Engine/EditorBlueprintResources/StandardMacros.IncrementInt` (`self.CurrentEtage`)))

(fn `MoveToDirection`
  (params (Direction :type "Vector Structure"))
  (`self.K2_SetActorLocation` (+ (`self.K2_GetActorLocation`) (* (`KismetMathLibrary.Normal` Direction) (0.0 0.0 300.0)))))

(fn `UserConstructionScript`)