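; BP_ElevatorTriggerDown is a trigger actor that sends a linked elevator down when the player character enters it.
; Overlapping its box prints a debug message, casts the other actor to BP_Character, then calls GoDown on the referenced Elevator.
; An unconnected leftover branch would toggle between GoUp and GoDown based on the elevator's IsDown state.
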(event `self.Box.OnComponentBeginOverlap`
  (params (OverlappedComponent :type "PrimitiveComponent Object Reference") (OtherActor :type "Actor Object Reference") (OtherComp :type "PrimitiveComponent Object Reference") (OtherBodyIndex :type Integer) (bFromSweep :type Boolean) (SweepResult :type "HitResult Structure (by ref)"))
  (`KismetSystemLibrary.PrintString` "Trigger Down Activé")
  (cast `/Game/Creation_Nicolas/BP_Character` OtherActor)
  (`/Game/Creation_Nicolas/BP_Elevator.GoDown` (`self.Elevator`)))

(fn `UserConstructionScript`)